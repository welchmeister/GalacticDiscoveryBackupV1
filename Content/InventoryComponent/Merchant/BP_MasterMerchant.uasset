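; BP_MasterMerchant is a merchant actor that holds a shop inventory and keeps interacting players' views of it in sync.
; CallAddItemtoInteractable appends an item the requested number of times, and ItemBought removes the first matching entry.
; After each single addition or removal, it pushes the whole MerchantInventory array to every interacting player's AC_InventoryComponent through UpdateMerchantInventory.
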(event `/Game/InventoryComponent/BPI_InventoryInterface.CallAddItemToInteractable`
  (params (`Item To add` :type "/Game/InventoryComponent/Items/BP_MasterInteractable Class Reference") (AmountToAdd :type Integer))
  (for _ (range 1 (+ AmountToAdd 1))
    (`KismetArrayLibrary.Array_Add` (`self.MerchantInventory`) `Item To add`)
    (for _array_element (`self.InteractingPlayers`)
      (`/Game/InventoryComponent/AC_InventoryComponent.UpdateMerchantInventory` (`self.GetComponentByClass` _array_element "/Game/InventoryComponent/AC_InventoryComponent.AC_InventoryComponent_C") (`self.MerchantInventory`)))))

(fn `ItemBought`
  (params (ItemToFind :type "/Game/InventoryComponent/Items/BP_MasterInteractable Class Reference (by ref)"))
  (`KismetArrayLibrary.Array_Remove` (`self.MerchantInventory`) (`KismetArrayLibrary.Array_Find` (`self.MerchantInventory`) ItemToFind))
  (for _array_element (`self.InteractingPlayers`)
    (`/Game/InventoryComponent/AC_InventoryComponent.UpdateMerchantInventory` (`self.GetComponentByClass` _array_element "/Game/InventoryComponent/AC_InventoryComponent.AC_InventoryComponent_C") (`self.MerchantInventory`))))

(fn `UserConstructionScript`
  (`parent.UserConstructionScript`))