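; TargetDummy is a damageable quest target that reports its objective ID to the player character when its health runs out, then hides its markers and destroys itself.
; On BeginPlay it creates a hidden compass marker after a short delay.
; Tick polls the player's current quests, toggling both markers on a hard-coded stage 2 check and feeding color and distance in meters to the in-world marker widget.
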(event `self.ReceiveBeginPlay`
  (bind _asmaster_character (cast `/Game/InventoryComponent/Demo/ThirdPerson/Blueprints/MasterCharacter` (`GameplayStatics.GetPlayerCharacter` 0)))
  (set `self.As Master Character` _asmaster_character)
  (`KismetSystemLibrary.Delay` 0.2)
  (bind _returnvalue (`|CreateWidget` "/Game/UserInterface/UI/wdg_compass_marker.wdg_compass_marker_C"))
  (bind _output_get (set `self.marker` _returnvalue))
  (`UserWidget.AddToViewport` (`self.marker`) 0)
  (`/Game/UserInterface/UI/wdg_compass_marker.Initialize_marker` _output_get "/Game/UserInterface/UI/MI_Marker.MI_Marker" (`self.marker color`) self)
  (`/Game/UserInterface/UI/wdg_compass_marker.Initialize_marker` (`self.marker`) "/Game/UserInterface/UI/MI_Marker.MI_Marker" (`self.marker color`) self)
  (`Widget.SetVisibility` (`self.marker`) "Hidden"))

(event `self.ReceiveTick`
  (params (DeltaSeconds :type "Float (single-precision)"))
  (bind _marker (`self.marker`))
  (bind _marker_widget (`self.Marker Widget`))
  (bind _marker_2 (`self.marker`))
  (bind _marker_widget_2 (`self.Marker Widget`))
  (for _array_element (`/Game/QuestSystem/QuestLogComponent.CurrentQuests` (`/Game/InventoryComponent/Demo/ThirdPerson/Blueprints/MasterCharacter.QuestLogComponent` (`self.As Master Character`)))
    (if (== (`/Game/QuestSystem/Quest_Base.CurrentStage` _array_element) 2)
      (`/Engine/EditorBlueprintResources/StandardMacros.IsValid` _marker_widget_2
        (:`Is Valid`
          (`SceneComponent.SetVisibility` _marker_widget_2 true false)
          (`/Engine/EditorBlueprintResources/StandardMacros.IsValid` _marker_2
            (:`Is Valid`
              (`Widget.SetVisibility` _marker_2 "Visible")
              (message `/Game/UserInterface/UI/BPI_MarkerWidget.UpdateText` (`WidgetComponent.GetUserWidgetObject` (`self.Marker Widget`)) (`KismetTextLibrary.Conv_StringToText` (`KismetStringLibrary.Concat_StrStr` (`KismetStringLibrary.Conv_IntToString` (`KismetMathLibrary.FTrunc` (/ (`KismetMathLibrary.Vector_Distance` (`self.K2_GetActorLocation`) (`self.K2_GetActorLocation` (`GameplayStatics.GetPlayerCharacter` 0))) 100.0))) "m")))
              (message `/Game/UserInterface/UI/BPI_MarkerWidget.SetMarkerColor` (`WidgetComponent.GetUserWidgetObject` (`self.Marker Widget`)) (`self.marker color`))))))
      (else
        (`/Engine/EditorBlueprintResources/StandardMacros.IsValid` _marker_widget
          (:`Is Valid`
            (`SceneComponent.SetVisibility` _marker_widget false false)
            (`/Engine/EditorBlueprintResources/StandardMacros.IsValid` _marker
              (:`Is Valid`
                (`Widget.SetVisibility` _marker "Hidden")))))))))

(event `self.ReceiveAnyDamage`
  (params (Damage :type "Float (single-precision)") (DamageType :type "DamageType Object Reference") (InstigatedBy :type "Controller Object Reference") (DamageCauser :type "Actor Object Reference"))
  (bind _marker (`self.marker`))
  (bind _marker_widget (`self.Marker Widget`))
  (`KismetSystemLibrary.PrintString` (`KismetStringLibrary.Conv_DoubleToString` Damage))
  (bind _output_get (set `self.Health` (- (`self.Health`) Damage)))
  (if (<= _output_get 0.0)
    (`/Game/InventoryComponent/Demo/ThirdPerson/Blueprints/MasterCharacter.OnObjectiveIDCalled` (`self.As Master Character`) (`self.ObjectiveID`) 1)
    (`/Engine/EditorBlueprintResources/StandardMacros.IsValid` _marker_widget
      (:`Is Valid`
        (`SceneComponent.SetVisibility` _marker_widget false false)
        (`/Engine/EditorBlueprintResources/StandardMacros.IsValid` _marker
          (:`Is Valid`
            (`Widget.SetVisibility` _marker "Hidden")
            (`self.K2_DestroyActor`)))))))

(fn `UserConstructionScript`)