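; LocationMarker is a quest objective actor that guides the player to a named location with a compass marker and a distance label.
; BeginPlay creates a hidden, color-tinted compass widget for the actor.
; Tick shows both markers while hardcoded quest "10001" is at stage 1, updating the distance in meters.
; Player overlap reports the objective ID, hides the markers and displays a location notification.
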(event `self.ReceiveBeginPlay`
  ;[1 1 1] BeginPlay
  (bind _asmaster_character (cast `/Game/InventoryComponent/Demo/ThirdPerson/Blueprints/MasterCharacter` (`GameplayStatics.GetPlayerCharacter` 0)))
  (set `self.As Master Character` _asmaster_character)
  (`KismetSystemLibrary.Delay` 0.2)
  (bind _returnvalue (`|CreateWidget` "/Game/UserInterface/UI/wdg_compass_marker.wdg_compass_marker_C"))
  (bind _output_get (set `self.marker` _returnvalue))
  (`UserWidget.AddToViewport` (`self.marker`) 0)
  (`/Game/UserInterface/UI/wdg_compass_marker.Initialize_marker` _output_get "/Game/UserInterface/UI/MI_Marker.MI_Marker" (`self.marker color`) self)
  (`/Game/UserInterface/UI/wdg_compass_marker.Initialize_marker` (`self.marker`) "/Game/UserInterface/UI/MI_Marker.MI_Marker" (`self.marker color`) self)
  (`Widget.SetVisibility` (`self.marker`) "Hidden"))

(event `self.ReceiveTick`
  (params (DeltaSeconds :type "Float (single-precision)"))
  (bind _markerwidget (`self.MarkerWidget`))
  (bind _marker (`self.marker`))
  (bind _marker_2 (`self.marker`))
  ;[1 1 1] Tick
  (bind _array_element (`/Game/QuestSystem/QuestLogComponent.GetQuestActor` (`/Game/InventoryComponent/Demo/ThirdPerson/Blueprints/MasterCharacter.QuestLogComponent` (`self.As Master Character`)) "10001"))
  (`/Engine/EditorBlueprintResources/StandardMacros.IsValid` _array_element
    (:`Is Valid`
      (if (== (`/Game/QuestSystem/Quest_Base.CurrentStage` _array_element) 1)
        (`/Engine/EditorBlueprintResources/StandardMacros.IsValid` _marker_2
          (:`Is Valid`
            (`Widget.SetVisibility` _marker_2 "Visible")
            (message `/Game/UserInterface/UI/BPI_MarkerWidget.UpdateText` (`WidgetComponent.GetUserWidgetObject` (`self.MarkerWidget`)) (`KismetTextLibrary.Conv_StringToText` (`KismetStringLibrary.Concat_StrStr` (`KismetStringLibrary.Conv_IntToString` (`KismetMathLibrary.FTrunc` (/ (`KismetMathLibrary.Vector_Distance` (`self.K2_GetActorLocation`) (`self.K2_GetActorLocation` (`GameplayStatics.GetPlayerCharacter` 0))) 100.0))) "m")))
            (message `/Game/UserInterface/UI/BPI_MarkerWidget.SetMarkerColor` (`WidgetComponent.GetUserWidgetObject` (`self.MarkerWidget`)) (`self.marker color`))
            (`SceneComponent.SetVisibility` (`self.MarkerWidget`) true false)))
        (else
          (`/Engine/EditorBlueprintResources/StandardMacros.IsValid` _markerwidget
            (:`Is Valid`
              (`SceneComponent.SetVisibility` _markerwidget false false)
              (`/Engine/EditorBlueprintResources/StandardMacros.IsValid` _marker
                (:`Is Valid`
                  (`Widget.SetVisibility` _marker "Hidden"))))))))))

(event `self.ReceiveActorBeginOverlap`
  (params (OtherActor :type "Actor Object Reference"))
  (bind _marker (`self.marker`))
  (bind _markerwidget (`self.MarkerWidget`))
  ;[1 1 1] Actor Begin Overlap
  (bind _asmaster_character (cast `/Game/InventoryComponent/Demo/ThirdPerson/Blueprints/MasterCharacter` OtherActor))
  (`/Game/InventoryComponent/Demo/ThirdPerson/Blueprints/MasterCharacter.OnObjectiveIDCalled` _asmaster_character (`self.ObjectiveID`) 1)
  (bind _returnvalue (`|CreateWidget` "/Game/UserInterface/LocationNotify.LocationNotify_C" null (`self.LocationName`)))
  (`/Engine/EditorBlueprintResources/StandardMacros.IsValid` _markerwidget
    (:`Is Valid`
      (`SceneComponent.SetVisibility` _markerwidget false false)
      (`/Engine/EditorBlueprintResources/StandardMacros.IsValid` _marker
        (:`Is Valid`
          (`Widget.SetVisibility` _marker "Hidden")
          (`UserWidget.AddToViewport` _returnvalue 0))))))

(fn `UserConstructionScript`)