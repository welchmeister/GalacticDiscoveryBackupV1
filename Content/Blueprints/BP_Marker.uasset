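; BP_Marker is a world marker actor that shows its distance from the player and registers itself on a compass bar.
; The construction script tints its cone with MarkerColor, and BeginPlay passes that color to the floating widget.
; After a short delay, it creates a compass marker widget, initialized with a material, the color and itself as owner.
; Each Tick updates the widget text with the distance in whole meters.
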(event `self.ReceiveBeginPlay`
  (bind _marker (`self.marker`))
  (`KismetSystemLibrary.Delay` 0.2)
  (bind _returnvalue (`|CreateWidget` "/Game/UserInterface/UI/wdg_compass_marker.wdg_compass_marker_C"))
  (bind _output_get (set `self.marker` _returnvalue))
  (`UserWidget.AddToViewport` _marker 0)
  (`/Game/UserInterface/UI/wdg_compass_marker.Initialize_marker` _marker "/Game/UserInterface/UI/MI_Marker.MI_Marker" (`self.marker color`) self)
  (`/Game/UserInterface/UI/wdg_compass_marker.Initialize_marker` _output_get "/Game/UserInterface/UI/MI_Marker.MI_Marker" (`self.marker color`) self)
  (message `/Game/UserInterface/UI/BPI_MarkerWidget.SetMarkerColor` (`WidgetComponent.GetUserWidgetObject` (`self.marker widget`)) (`self.marker color`)))

(event `self.ReceiveTick`
  (params (DeltaSeconds :type "Float (single-precision)"))
  (message `/Game/UserInterface/UI/BPI_MarkerWidget.UpdateText` (`WidgetComponent.GetUserWidgetObject` (`self.marker widget`)) (`KismetTextLibrary.Conv_StringToText` (`KismetStringLibrary.Concat_StrStr` (`KismetStringLibrary.Conv_IntToString` (`KismetMathLibrary.FTrunc` (/ (`KismetMathLibrary.Vector_Distance` (`self.K2_GetActorLocation`) (`self.K2_GetActorLocation` (`GameplayStatics.GetPlayerCharacter` 0))) 100.0))) "m"))))

(fn `UserConstructionScript`
  (`MeshComponent.SetVectorParameterValueOnMaterials` (`self.Cone`) "Color" (`KismetMathLibrary.Conv_LinearColorToVector` (`self.marker color`))))