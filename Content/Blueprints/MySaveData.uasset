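; MySaveData is a save data object that stores and restores the player's quest state.
; SaveQuestLog copies the active and completed quest lists from a quest log, while SaveQuestDetails records each quest's stage and objective progress in a map keyed by quest ID.
; LoadQuests re-adds each active quest through the quest log component, applies its saved stage and progress, then overwrites the component's active and completed lists.
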(fn `LoadQuests`
  (params (`Quest Log Component` :type "/Game/QuestSystem/QuestLogComponent Object Reference"))
  (for _array_element (`self.CurrentActiveQuests`)
    (bind _returnvalue (`/Game/QuestSystem/QuestLogComponent.AddNewQuest` `Quest Log Component` _array_element))
    (bind (_progress _currentstage) (break `/Game/QuestSystem/FQuestSaveData` (`BlueprintMapLibrary.Map_Find` (`self.QuestProgress`) _array_element)))
    (set `/Game/QuestSystem/Quest_Base.CurrentStage` _currentstage _returnvalue)
    (set `/Game/QuestSystem/Quest_Base.CurrentObjectiveProgress` _progress _returnvalue))
  (set `/Game/QuestSystem/QuestLogComponent.CurrentActiveQuests` (`self.CurrentActiveQuests`) `Quest Log Component`)
  (set `/Game/QuestSystem/QuestLogComponent.CompletedQuests` (`self.CompletedQuests`) `Quest Log Component`))

(fn `SaveQuestDetails`
  (params (Quest :type "/Game/QuestSystem/Quest_Base Object Reference"))
  (`BlueprintMapLibrary.Map_Add` (`self.QuestProgress`) (`/Game/QuestSystem/Quest_Base.QuestID` Quest) (make `/Game/QuestSystem/FQuestSaveData` (`/Game/QuestSystem/Quest_Base.CurrentObjectiveProgress` Quest) (`/Game/QuestSystem/Quest_Base.CurrentStage` Quest))))

(fn `SaveQuestLog`
  (params (`Quest Log` :type "/Game/QuestSystem/QuestLogComponent Object Reference"))
  (set `self.CurrentActiveQuests` (`/Game/QuestSystem/QuestLogComponent.CurrentActiveQuests` `Quest Log`))
  (set `self.CompletedQuests` (`/Game/QuestSystem/QuestLogComponent.CompletedQuests` `Quest Log`)))