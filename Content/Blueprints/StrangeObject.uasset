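; StrangeObject is an interactable quest-objective actor that identifies itself as "strangeobject" and guides the player to it with markers.
; BeginPlay creates a hidden compass marker after a short delay and reads stages from the player's active quests.
; Tick loops over current quests, showing the compass marker and a widget with player distance in meters for stage 0 while the quest tracker is visible, otherwise hiding them.
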(event `self.ReceiveBeginPlay`
  (bind _questlogcomponent (`/Game/InventoryComponent/Demo/ThirdPerson/Blueprints/MasterCharacter.QuestLogComponent` (`self.As Master Character`)))
  (bind _asmaster_character (cast `/Game/InventoryComponent/Demo/ThirdPerson/Blueprints/MasterCharacter` (`GameplayStatics.GetPlayerCharacter` 0)))
  (set `self.As Master Character` _asmaster_character)
  (`KismetSystemLibrary.Delay` 0.2)
  (bind _returnvalue (`|CreateWidget` "/Game/UserInterface/UI/wdg_compass_marker.wdg_compass_marker_C"))
  (bind _output_get (set `self.marker` _returnvalue))
  (`UserWidget.AddToViewport` (`self.marker`) 0)
  (`/Game/UserInterface/UI/wdg_compass_marker.Initialize_marker` _output_get "/Game/UserInterface/UI/MI_Marker.MI_Marker" (`self.marker color`) self)
  (`/Game/UserInterface/UI/wdg_compass_marker.Initialize_marker` (`self.marker`) "/Game/UserInterface/UI/MI_Marker.MI_Marker" (`self.marker color`) self)
  (`Widget.SetVisibility` (`self.marker`) "Hidden")
  (for _array_element (`/Game/QuestSystem/QuestLogComponent.CurrentActiveQuests` _questlogcomponent)
    (bind _array_element_2 (`/Game/QuestSystem/QuestLogComponent.GetQuestActor` _questlogcomponent _array_element))
    (set `self.CurrentStage` (`/Game/QuestSystem/Quest_Base.CurrentStage` _array_element_2))))

(event `self.ReceiveTick`
  (params (DeltaSeconds :type "Float (single-precision)"))
  (bind _markerwidget (`self.MarkerWidget`))
  (bind _marker (`self.marker`))
  (bind _marker_2 (`self.marker`))
  (bind _questlogcomponent (`/Game/InventoryComponent/Demo/ThirdPerson/Blueprints/MasterCharacter.QuestLogComponent` (`self.As Master Character`)))
  (bind _tracker (`/Game/QuestSystem/QuestLogComponent.Tracker` _questlogcomponent))
  (`/Engine/EditorBlueprintResources/StandardMacros.IsValid` _tracker
    (:`Is Valid`
      (for _array_element (`/Game/QuestSystem/QuestLogComponent.CurrentQuests` _questlogcomponent)
        (if (and (== (`/Game/QuestSystem/Quest_Base.CurrentStage` _array_element) 0) (`Widget.IsVisible` _tracker))
          (`/Engine/EditorBlueprintResources/StandardMacros.IsValid` _marker_2
            (:`Is Valid`
              (`Widget.SetVisibility` _marker_2 "Visible")
              (message `/Game/UserInterface/UI/BPI_MarkerWidget.UpdateText` (`WidgetComponent.GetUserWidgetObject` (`self.MarkerWidget`)) (`KismetTextLibrary.Conv_StringToText` (`KismetStringLibrary.Concat_StrStr` (`KismetStringLibrary.Conv_IntToString` (`KismetMathLibrary.FTrunc` (/ (`KismetMathLibrary.Vector_Distance` (`self.K2_GetActorLocation`) (`self.K2_GetActorLocation` (`GameplayStatics.GetPlayerCharacter` 0))) 100.0))) "m")))
              (message `/Game/UserInterface/UI/BPI_MarkerWidget.SetMarkerColor` (`WidgetComponent.GetUserWidgetObject` (`self.MarkerWidget`)) (`self.marker color`))
              (`SceneComponent.SetVisibility` (`self.MarkerWidget`) true false)))
          (else
            (`/Engine/EditorBlueprintResources/StandardMacros.IsValid` _markerwidget
              (:`Is Valid`
                (`SceneComponent.SetVisibility` _markerwidget false false)
                (`/Engine/EditorBlueprintResources/StandardMacros.IsValid` _marker
                  (:`Is Valid`
                    (`Widget.SetVisibility` _marker "Hidden")))))))))))

(fn `InteractWith`
  (returns (ObjectiveID :type String))
  (return "strangeobject"))

(fn `UserConstructionScript`)