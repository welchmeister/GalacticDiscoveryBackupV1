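; Inventory component that stores item quantities in a Content map, with functions to add, remove and query items.
; Add and Remove overwrite the map entry with the adjusted count, with no clamping or removal of empty entries.
; Both then fire the player MasterCharacter's OnObjectiveIDCalled dispatcher with the item as ID and the signed quantity change, letting objective listeners react to inventory changes.
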(fn `AddToInventory`
  (params (Item :type Name) (Quantity :type Integer))
  (`BlueprintMapLibrary.Map_Add` (`self.Content`) Item (+ Quantity (`BlueprintMapLibrary.Map_Find` (`self.Content`) Item)))
  (bind _asmaster_character (cast `/Game/InventoryComponent/Demo/ThirdPerson/Blueprints/MasterCharacter` (`GameplayStatics.GetPlayerCharacter` 0)))
  (`/Game/InventoryComponent/Demo/ThirdPerson/Blueprints/MasterCharacter.OnObjectiveIDCalled` _asmaster_character (`KismetStringLibrary.Conv_NameToString` (`local.Item`)) (`local.Quantity`)))

(fn `QueryInventory`
  (params (Item :type Name))
  (returns (Value :type Integer))
  (return (`BlueprintMapLibrary.Map_Find` (`self.Content`) Item)))

(fn `RemoveFromInventory`
  (params (Item :type "Name (by ref)") (Quantity :type Integer))
  (`BlueprintMapLibrary.Map_Add` (`self.Content`) Item (- (`BlueprintMapLibrary.Map_Find` (`self.Content`) Item) Quantity))
  (bind _asmaster_character (cast `/Game/InventoryComponent/Demo/ThirdPerson/Blueprints/MasterCharacter` (`GameplayStatics.GetPlayerCharacter` 0)))
  (`/Game/InventoryComponent/Demo/ThirdPerson/Blueprints/MasterCharacter.OnObjectiveIDCalled` _asmaster_character (`KismetStringLibrary.Conv_NameToString` (`local.Item`)) (* (`local.Quantity`) -1)))